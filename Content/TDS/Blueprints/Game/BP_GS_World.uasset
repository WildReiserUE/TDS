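; World game state (by its GS prefix) that tracks player lives, experience, best score and stage progression for the current level.
; On BeginPlay it finds the DT_Levels row matching the level name and copies its phase thresholds and best score.
; Respawn checks spend a life, except on first start, and report success with the stage.
; Added experience raises the best score and advances one stage per exceeded threshold, returning true after the last.
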(event EventBeginPlay
  (bind _returnvalue (Game|GetCurrentLevelName true))
  (bind _outrownames (DataTable|GetDataTableRowNames "/Game/TDS/Blueprints/Game/DT_Levels.DT_Levels"))
  (bind _array_element (Utilities|Array|ForEachLoopwithBreak _outrownames :!label _label)
    (:LoopBody
      (bind _returnvalue_2 (Utilities|GetDataTableRow "/Game/TDS/Blueprints/Game/DT_Levels.DT_Levels" _array_element)
        (:then
          (if (Utilities|Name|Equal(Name) (.LevelName (Utilities|Struct|BreakS_Levels _returnvalue_2)) (Utilities|String|StringToName _returnvalue))
            (Variables|Default|SetPhase%20Value (.PhaseValue (Utilities|Struct|BreakS_Levels _returnvalue_2)))
            (Variables|Default|SetBest%20Score (.BestScore (Utilities|Struct|BreakS_Levels _returnvalue_2)))
            (goto _label Break)))))))

(fn ConstructionScript)

(fn CanPlayerRespawn
  (bind _playerlives (Variables|Default|GetPlayerLives))
  (bind _currentstage (Variables|Default|GetCurrentStage))
  (bind _returnvalue (>= _playerlives 0))
  (if (and (Variables|Default|GetbFirstStart) _returnvalue)
    (bind _output_get (Variables|Default|SetbFirstStart (Variables|Default|GetbFirstStart)))
    (if _output_get
      (Variables|Default|SetbFirstStart false)
      (return _returnvalue _currentstage)
      (else
        _))
    (elif _returnvalue
      _
      (else
        (return false 0))))
  (Math|Integer|DecrementInt _playerlives
    (:%20%20
      (return _returnvalue _currentstage))))

(fn GetPlayerCanRestart
  (return (Variables|Default|GetbFirstStart)))

(fn ExperienceCalculate
  (params (AddExperience :type Integer))
  (bind _output_get (Variables|Default|SetPlayerExperience (+ (Variables|Default|GetPlayerExperience) AddExperience)))
  (if (> _output_get (Variables|Default|GetBest%20Score))
    (Variables|Default|SetBest%20Score _output_get))
  (if (< (Utilities|Array|Get(acopy) (Variables|Default|GetPhase%20Value) (Variables|Default|GetCurrentStage)) (Variables|Default|GetPlayerExperience))
    (if (Utilities|Array|IsValidIndex (Variables|Default|GetPhase%20Value) (+ (Variables|Default|GetCurrentStage) 1))
      (Variables|Default|SetCurrentStage (+ (Variables|Default|GetCurrentStage) 1))
      (else
        (return true)))))