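; Player controller for the game world that owns the HUD and drives the spawn, death and restart flow.
; On start or restart it asks BP_GM_World to respawn, possesses the character and creates W_GameMain.
; Once character components are added, health, inventory, weapon and sprint delegates update the HUD.
; It also handles minimap zoom, the Q options menu and the end-game screen with restart, menu or quit.
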(event Custom|ClickZoomIn_Event_0
  (bind _scenecapturecomponent2d (Variables|Default|GetSceneCaptureComponent2D))
  ;[0 0 0] MinimapControl
  (Variables|/Script/Engine.SceneCaptureComponent2D|SetOrthoWidth _scenecapturecomponent2d (Math|Float|Clamp(Float) (- (Variables|/Script/Engine.SceneCaptureComponent2D|GetOrthoWidth _scenecapturecomponent2d) 3e+02) 1.6e+03 3.7e+03)))

(event Custom|ClickZoomOut_Event_0
  (bind _scenecapturecomponent2d (Variables|Default|GetSceneCaptureComponent2D))
  ;[0 0 0] MinimapControl
  (Variables|/Script/Engine.SceneCaptureComponent2D|SetOrthoWidth _scenecapturecomponent2d (Math|Float|Clamp(Float) (+ (Variables|/Script/Engine.SceneCaptureComponent2D|GetOrthoWidth _scenecapturecomponent2d) 3e+02) 1.6e+03 3.7e+03)))

(event Custom|SwitchWeapon
  (params (WeaponIndex :type Integer))
  ;[1 1 1] Character Events
  (Default|UpdateActiveWeapon (Variables|/Game/TDS/UI/UI_Game/W_GameMain.W_GameMain_C|GetW_WeaponPanel (Variables|Default|GetW_GameWidget)) WeaponIndex)
  (EventDispatchers|AssignOnWeaponFire (Variables|/Script/TDS.BaseCharacter|GetCurrentWeapon (Variables|Default|GetBPTDPCharacter)) (delegate Custom|OnWeaponFire_Event_0)))

(event Custom|Click_ToMenu_Event_0
  ;[0 0 0] HEAL EVENTS
  (Widget|RemovefromParent (Variables|Default|GetW_GameWidget))
  (Game|OpenLevel(byName) "MainMenu"))

(event Custom|Again
  ;[0 0 0] Смеркалось
  (Audio|PushSoundMixModifier "/Game/TDS/Audio/BP_SoundMix.BP_SoundMix")
  (bind _asbp_gm_world (Utilities|Casting|CastToBP_GM_World (Game|GetGameMode)))
  (bind _success (Default|TrytoRespawn _asbp_gm_world))
  (if _success
    (bind _asbp_tdscharacter (Utilities|Casting|CastToBP_TDSCharacter (Game|Player|GetPlayerPawn 0)))
    (bind _output_get (Variables|Default|SetBPTDPCharacter _asbp_tdscharacter))
    (Pawn|Possess _output_get)
    (CallFunction|PlayStep2)))

(event Custom|MakeMinimapControl
  (params (W_Minimap :type W%20Minimap%20Object%20Reference))
  ;[0 0 0] MinimapControl
  (EventDispatchers|AssignClickZoomin W_Minimap (delegate Custom|ClickZoomIn_Event_0))
  (EventDispatchers|AssignClickZoomOut W_Minimap (delegate Custom|ClickZoomOut_Event_0)))

(event Custom|OnBulletsChanged_Event_0
  (params (Magazine :type Integer) (InventoryBullet :type Integer))
  (bind _w_gamewidget (Variables|Default|GetW_GameWidget))
  (bind _w_weaponpanel (Variables|/Game/TDS/UI/UI_Game/W_GameMain.W_GameMain_C|GetW_WeaponPanel _w_gamewidget))
  ;[1 1 1] Inventory Events
  (Default|UpdateActiveMagazine _w_weaponpanel Magazine)
  (Default|UpdateActiveInventory _w_weaponpanel InventoryBullet))

(event Custom|PlayStep2
  ;[0 0 0] Part.2
  (bind _gamewidget (CallFunction|CreateGameWidget self))
  (CallFunction|MakeMinimapControl (Variables|/Game/TDS/UI/UI_Game/W_GameMain.W_GameMain_C|GetW_Minimap _gamewidget))
  ;[0 0 0] HEAL EVENTS
  (EventDispatchers|AssignComponentsAdded (Variables|Default|GetBPTDPCharacter) (delegate Custom|ComponentsAdded_Event_0)))

(event Custom|OnPlayerFindItem_Event_0
  (params (ItemInfo :type Item%20Info%20Structure))
  ;[1 1 1] Inventory Events
  (Default|UpdateWidgetInfo (Variables|/Game/TDS/UI/UI_Game/W_GameMain.W_GameMain_C|GetW_WeaponPanel (Variables|Default|GetW_GameWidget)) ItemInfo (Variables|/Script/TDS.TDSInventory|GetInventory (Actor|GetComponentbyClass (Variables|Default|GetBPTDPCharacter) "/Script/TDS.TDSInventory"))))

(event Custom|InventoryEvents
  (bind _bptdpcharacter (Variables|Default|GetBPTDPCharacter))
  (bind _returnvalue (Actor|GetComponentbyClass _bptdpcharacter "/Script/TDS.TDSInventory"))
  ;[1 1 1] Inventory Events
  (EventDispatchers|AssignOnReloadEnd _returnvalue (delegate Custom|OnBulletsChanged_Event_0))
  (EventDispatchers|AssignOnFindItem _returnvalue (delegate Custom|OnPlayerFindItem_Event_0))
  (EventDispatchers|AssignOnCountChange _returnvalue (delegate Custom|OnCountChange_Event_0)))

(event Custom|SkillEvents
  ;[1 1 1] Skill Events
  (EventDispatchers|AssignOnSprintValueChange (Actor|GetComponentbyClass (Variables|Default|GetBPTDPCharacter) "/Script/TDS.TDSSkillComponent") (delegate Custom|OnSprintChange)))

(event Custom|CharacterEvents
  ;[1 1 1] Character Events
  (EventDispatchers|BindEventtoOnWeaponSwitch (Variables|Default|GetBPTDPCharacter) (delegate Custom|SwitchWeapon)))

(event Custom|OnShieldChange_Event_0
  (params (Shield :type Float%20%28single-precision%29) (MaxShield :type Float%20%28single-precision%29))
  ;[0 0 0] HEAL EVENTS
  (Default|FillShieldValue (Variables|Default|GetW_GameWidget) Shield MaxShield))

(event Custom|OnCountChange_Event_0
  (params (ItemCount :type Integer))
  ;[1 1 1] Inventory Events
  (Default|UpdateActiveInventory (Variables|/Game/TDS/UI/UI_Game/W_GameMain.W_GameMain_C|GetW_WeaponPanel (Variables|Default|GetW_GameWidget)) ItemCount))

(event Custom|OnWeaponFire_Event_0
  (params (Count :type Integer))
  ;[1 1 1] Character Events
  (Default|UpdateActiveMagazine (Variables|/Game/TDS/UI/UI_Game/W_GameMain.W_GameMain_C|GetW_WeaponPanel (Variables|Default|GetW_GameWidget)) Count))

(event Custom|OnHealthChange_Event_0
  (params (Health :type Float%20%28single-precision%29) (MaxHealth :type Float%20%28single-precision%29))
  ;[0 0 0] HEAL EVENTS
  (Default|FillHealthValue (Variables|Default|GetW_GameWidget) Health MaxHealth))

(event Custom|ComponentsAdded_Event_0
  (bind _bptdpcharacter (Variables|Default|GetBPTDPCharacter))
  (bind _returnvalue (Actor|GetComponentbyClass _bptdpcharacter "/Script/TDS.TDSHealthComponent"))
  ;[0 0 0] HEAL EVENTS
  (EventDispatchers|AssignOnShieldChange _returnvalue (delegate Custom|OnShieldChange_Event_0))
  (EventDispatchers|AssignOnHealthChange _returnvalue (delegate Custom|OnHealthChange_Event_0))
  (EventDispatchers|BindEventtoOnOwnerDeath _returnvalue (delegate Custom|CharDeath_Event))
  (CallFunction|InventoryEvents)
  (CallFunction|CharacterEvents)
  (CallFunction|SkillEvents))

(event Custom|CharDeath_Event
  (bind _bptdpcharacter (Variables|Default|GetBPTDPCharacter))
  (bind _characterinfo (Variables|/Script/TDS.BaseCharacter|GetCharacterInfo _bptdpcharacter))
  (bind _montagedead (Utilities|Struct|BreakBaseHumanoidData _characterinfo))
  ;[0 0 0] HEAL EVENTS
  (Widget|RemovefromParent (Variables|Default|GetW_GameWidget))
  (if (> (Utilities|Array|Length _montagedead) 0)
    (Animation|Montage|PlayMontage (Variables|/Script/Engine.Character|GetMesh _bptdpcharacter) (.OutItem (Utilities|Array|Random _montagedead))
      (:then
        (EventDispatchers|UnbindallEventsfromOnEndPlay _bptdpcharacter))))
  (bind _returnvalue (UserInterface|CreateWidget "/Game/TDS/UI/UI_Game/W_EndGame.W_EndGame_C"))
  (bind _output_get (Variables|Default|SetDeadWidget _returnvalue))
  (UserInterface|Viewport|AddtoViewport _output_get 0)
  (EventDispatchers|AssignClickRestart _output_get (delegate Custom|Click_Yes_Event_0))
  (EventDispatchers|AssignClickNo _output_get (delegate Custom|Click_No_Event_0))
  (EventDispatchers|AssignClicktoMenu _output_get (delegate Custom|Click_ToMenu_Event_0)))

(event Custom|Click_Yes_Event_0
  ;[0 0 0] HEAL EVENTS
  (EventDispatchers|UnbindEventfromClickRestart (stale Custom|CharDeath_Event _output_get) (delegate Custom|Click_Yes_Event_0))
  (Widget|RemovefromParent (stale Custom|CharDeath_Event _output_get))
  (Pawn|UnPossess)
  (CallFunction|Again))

(event Custom|Click_No_Event_0
  ;[0 0 0] HEAL EVENTS
  (Game|QuitGame 0 "Quit" false))

(event Custom|OnSprintChange
  (params (CurrentSprintValue :type Float%20%28single-precision%29) (MaxSprintValue :type Float%20%28single-precision%29))
  ;[1 1 1] Skill Events
  (Default|FillStaminaValue (Variables|Default|GetW_GameWidget) CurrentSprintValue MaxSprintValue))

(event Custom|Click_X_Event_0
  ;[0 0 0] Options
  (Widget|SetVisibility (Variables|/Game/TDS/UI/UI_Game/W_GameMain.W_GameMain_C|GetOptions_Box (Variables|Default|GetW_GameWidget)) "Hidden"))

(event EventBeginPlay
  ;[0 0 0] Смеркалось
  (Audio|PushSoundMixModifier "/Game/TDS/Audio/BP_SoundMix.BP_SoundMix")
  (bind _asbp_gm_world (Utilities|Casting|CastToBP_GM_World (Game|GetGameMode)))
  (bind _success (Default|TrytoRespawn _asbp_gm_world))
  (if _success
    (bind _asbp_tdscharacter (Utilities|Casting|CastToBP_TDSCharacter (Game|Player|GetPlayerPawn 0)))
    (bind _output_get (Variables|Default|SetBPTDPCharacter _asbp_tdscharacter))
    (Pawn|Possess _output_get)
    (CallFunction|PlayStep2)))

(event Input|KeyboardEvents|Q
  (params (Key :type Key%20Structure :default "None"))
  (bind _w_gamewidget (Variables|Default|GetW_GameWidget))
  (bind _options_box (Variables|/Game/TDS/UI/UI_Game/W_GameMain.W_GameMain_C|GetOptions_Box _w_gamewidget))
  ;[0 0 0] Options
  (:Pressed
    (if (Widget|IsVisible _options_box)
      (Widget|SetVisibility _options_box "Hidden")
      (else
        (EventDispatchers|AssignClickX (Variables|/Game/TDS/UI/UI_Game/W_GameMain.W_GameMain_C|GetW_OptionsMenu _w_gamewidget) (delegate Custom|Click_X_Event_0))
        (Widget|SetVisibility _options_box "Visible")))))

(fn ConstructionScript)

(fn CreateGameWidget
  (params (OwningPlayer :type Player%20Controller%20Object%20Reference))
  (bind _returnvalue (UserInterface|CreateWidget "/Game/TDS/UI/UI_Game/W_GameMain.W_GameMain_C" OwningPlayer))
  (bind _output_get (Variables|Default|SetW_GameWidget _returnvalue))
  (UserInterface|Viewport|AddtoViewport _output_get 0)
  (return _output_get))