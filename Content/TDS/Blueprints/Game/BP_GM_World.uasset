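; BP_GM_World is the world game mode, handling player spawning, stage-based respawning and the win screen on top of BP_GS_World.
; Players first spawn at the "Stage1" start; TryToRespawn asks the game state for permission and restarts player 0 at the current stage's tagged start, returning success.
; PlayerExp forwards experience to the game state and shows the W_EndGame win widget when that check passes.
; WinExperienceRules is an empty stub.
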(fn ConstructionScript)

(fn TrytoRespawn
  (bind _returnvalue (Game|GetPlayerController 0))
  (bind _asbp_gs_world (Utilities|Casting|CastToBP_GS_World (Game|GetGameState)))
  (bind (_bissuccess _currentstage) (Default|CanPlayerRespawn _asbp_gs_world))
  (if _bissuccess
    (Class|GameModeBase|RestartPlayeratPlayerStart _returnvalue (Class|GameModeBase|FindPlayerStart _returnvalue (Utilities|Select :Index _currentstage :Option%200 "Stage1" :Option%201 "Stage2" :Option%202 "Stage3" :Option%203 "Stage4")))
    (return true)
    (else
      (return false))))

(fn ChoosePlayerStart
  (params (Player :type Controller%20Object%20Reference))
  (return (Class|GameModeBase|FindPlayerStart Player "Stage1")))

(fn PlayerExp
  (params (Experience :type Integer))
  (bind _asbp_gs_world (Utilities|Casting|CastToBP_GS_World (Game|GetGameState)))
  (bind _biswin_ (Default|ExperienceCalculate _asbp_gs_world Experience))
  (if _biswin_
    (bind _returnvalue (UserInterface|CreateWidget "/Game/TDS/UI/UI_Game/W_EndGame.W_EndGame_C" (Game|GetPlayerController 0) true))
    (UserInterface|Viewport|AddtoViewport _returnvalue 0)))

(fn WinExperienceRules
  (params (Score :type Integer)))