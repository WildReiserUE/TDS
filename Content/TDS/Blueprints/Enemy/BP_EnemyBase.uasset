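; Base enemy character that configures itself from the DT_NPC data table row matching its NPCId.
; The construction script applies name, mesh, animation class, speed, health, shield, mana and experience, with a fallback name for missing rows.
; BeginPlay shows a name widget where cosmetics run, and animation-finish events clear the damage widget or hide and destroy the actor.
; Damage-number and death-experience chains are unwired, and GetPhisMat is an empty stub.
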(event Custom|AnimFinish_1
  (Rendering|SetVisibility (Variables|Character|GetMesh) false false)
  (Utilities|FlowControl|Delay 1.0)
  (Actor|DestroyActor))

(event Custom|AnimFinished_Event_0
  (UserInterface|SetWidget (Variables|Default|GetDamageWidget) 0))

(event EventBeginPlay
  (Networking|CanExecuteCosmeticEvents
    (:True
      (bind _returnvalue (UserInterface|CreateWidget "/Game/TDS/UI/UI_Game/W_CharName.W_CharName_C"))
      (bind _output_get (Variables|Default|SetUpperWidget _returnvalue))
      (UserInterface|SetWidget (Variables|Default|GetNameWidget) _output_get)
      (Variables|/Game/TDS/UI/UI_Game/W_CharName.W_CharName_C|SetWidgetName _output_get (Variables|Default|GetEnemyName)))))

(fn ConstructionScript
  (bind _mesh (Variables|Character|GetMesh))
  (bind _mesh_2 (Variables|Character|GetMesh))
  (bind _returnvalue (Utilities|GetDataTableRow "/Game/TDS/Blueprints/Enemy/DT_NPC.DT_NPC" (Variables|Default|GetNPC_Id))
    (:then
      (Variables|Default|SetEnemyName (.WidgetName (Utilities|Struct|BreakS_NPC_Data _returnvalue)))
      (Class|SkinnedMeshComponent|SetSkeletalMesh _mesh_2 (.SK_Mesh (Utilities|Struct|BreakS_NPC_Data _returnvalue)) true)
      (Class|SkeletalMeshComponent|SetAnimClass _mesh_2 (.SK_Anim (Utilities|Struct|BreakS_NPC_Data _returnvalue)))
      (Variables|Default|SetMana (.Mana (Utilities|Struct|BreakS_NPC_Data _returnvalue)))
      (Variables|/Script/Engine.CharacterMovementComponent|SetMaxWalkSpeed (Variables|Character|GetCharacterMovement) (.Walk_Speed (Utilities|Struct|BreakS_NPC_Data _returnvalue)))
      (Variables|Default|SetbCanUseShield (.bCanUseShield (Utilities|Struct|BreakS_NPC_Data _returnvalue)))
      (Variables|Default|SetMax%20Shield (.MaxShield (Utilities|Struct|BreakS_NPC_Data _returnvalue)))
      (Variables|Default|SetMaxHealth (.MaxHealth (Utilities|Struct|BreakS_NPC_Data _returnvalue)))
      (Variables|Default|SetShield%20Recovery%20Value (.ShieldRecoveryValue (Utilities|Struct|BreakS_NPC_Data _returnvalue)))
      (Variables|Default|SetShield%20Recovery%20Period (.ShieldRecoveryPeriod (Utilities|Struct|BreakS_NPC_Data _returnvalue)))
      (Variables|Default|SetExperience (.Experience (Utilities|Struct|BreakS_NPC_Data _returnvalue))))
    (:RowNotFound
      (Variables|Default|SetEnemyName "Unknow EnemyData NotFound")
      (Class|SkinnedMeshComponent|SetSkeletalMesh _mesh 0 true)
      (Class|SkeletalMeshComponent|SetAnimClass _mesh))))

(fn GetPhisMat
  (params (PhysMat :type Physical%20Material%20Object%20Reference))
  (return 0 0))