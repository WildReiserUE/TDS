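; BP_Door is a door that moves vertically when a Pawn overlaps its TriggerOut component, then returns automatically after a short delay.
; The OpenClose timeline drives the actor's Z offset from its starting height, and a separate Rreverse timeline later applies its own offset from the opened height.
; An IsOpen flag ignores overlaps until the cycle ends, when the flag and the DoOnce guarding the return are reset.
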(event OnComponentBeginOverlap(TriggerOut)
  (params (OverlappedComponent :type Primitive%20Component%20Object%20Reference) (OtherActor :type Actor%20Object%20Reference) (OtherComp :type Primitive%20Component%20Object%20Reference) (OtherBodyIndex :type Integer) (bFromSweep :type Boolean) (SweepResult :type Hit%20Result%20Structure%20%28by%20ref%29))
  (bind _returnvalue (Transformation|GetActorLocation))
  (Utilities|Casting|CastToPawn OtherActor)
  (if (not (Variables|Default|GetbIsOpen?))
    (Variables|Default|SetbIsOpen? true)
    (Variables|Default|SetLocZToStart (.z _returnvalue))
    (bind _z (Timeline|Open-Close PlayFromStart)
      (:Update
        (Transformation|SetActorLocation (Math|Vector|MakeVector (.x _returnvalue) (.y _returnvalue) (+ (Variables|Default|GetLocZToStart) _z)) false false))
      (:Finished
        (Utilities|FlowControl|Delay 3.0)
        (Utilities|FlowControl|DoOnce false :!label _label
          (:Completed
            (bind _output_get (Variables|Default|SetLocZToStart (+ (Variables|Default|GetLocZToStart) _z)))
            (bind _z_2 (Timeline|Rreverse PlayFromStart)
              (:Update
                (Transformation|SetActorLocation (Math|Vector|MakeVector (.x _returnvalue) (.y _returnvalue) (+ _output_get _z_2)) false false))
              (:Finished
                (Variables|Default|SetbIsOpen? false)
                (Variables|Default|SetLocZToStart (.z _returnvalue))
                (goto _label Reset)))))))))

(fn ConstructionScript)