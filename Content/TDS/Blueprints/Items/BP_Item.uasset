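; BP_Item is an item Blueprint that fills in its own data from the DT_Items data table.
; Its Construction Script looks up the row named by ItemID and switches on item type to store the matching weapon, armor or projectile info, with plain items needing none.
; It then stores the shared base info as ItemInfo and prints the item's name and type.
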(fn ConstructionScript
  (bind _returnvalue (Utilities|GetDataTableRow "/Game/TDS/Blueprints/Items/DT_Items.DT_Items" (Variables|Default|GetItemID))
    (:then
      (switch Utilities|FlowControl|Switch|SwitchonEItemType (.ItemType (Utilities|Struct|BreakS_ItemInfo _returnvalue))
        (:Item
          _)
        (:Weapon
          (Variables|Default|SetWeaponInfo (.WeaponInfo (Utilities|Struct|BreakS_ItemInfo _returnvalue))))
        (:Armor
          (Variables|Default|SetArmorInfo (.ArmorInfo (Utilities|Struct|BreakS_ItemInfo _returnvalue))))
        (:Projectile
          (Variables|Default|SetProjectileInfo (.ProjectileInfo (Utilities|Struct|BreakS_ItemInfo _returnvalue)))))
      (bind _output_get (Variables|Default|SetItemInfo (.BaseInfo (Utilities|Struct|BreakS_ItemInfo _returnvalue))))
      (Development|PrintString (Utilities|String|Append (Utilities|String|ToString(Name) (.ItemName (Utilities|Struct|BreakItemInfo _output_get))) "--" (Utilities|String|EnumtoString (.ItemType (Utilities|Struct|BreakItemInfo _output_get))))))))