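; BP_TDSCharacter is a TDS character Blueprint that assembles its components at runtime and sets up its camera arm.
; BeginPlay adds each class in ComponentList as a component, then calls ComponentAdded once all are created.
; The construction script copies the character's camera lag settings onto CameraArm.
; The T key serves as a debug dump, printing each TDSInventory item's ID, name and count, or EMPTY.
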(event EventBeginPlay
  (for _array_element (Variables|Default|GetComponentList)
    (Game|AddComponentbyClass _array_element))
  (Default|CallComponentAdded))

(event Input|KeyboardEvents|T
  (params (Key :type Key%20Structure :default "None"))
  (bind _returnvalue (Actor|GetComponentbyClass "/Script/TDS.TDSInventory"))
  (bind _inventory (Variables|/Script/TDS.TDSInventory|GetInventory _returnvalue))
  (:Pressed
    (if (> (Utilities|Array|Length _inventory) 0)
      (for _array_element _inventory
        (Development|PrintString (Utilities|String|Append (Utilities|String|ToString(Integer) (.ItemID (Utilities|Struct|BreakItemInfo _array_element))) "---" (Utilities|String|ToString(Name) (.ItemName (Utilities|Struct|BreakItemInfo _array_element))) "---" (Utilities|String|ToString(Integer) (.Count (Utilities|Struct|BreakItemInfo _array_element))))))
      (else
        (Development|PrintString "EMPTY")))))

(fn ConstructionScript
  (bind _cameraarm (Variables|Default|GetCameraArm))
  (Variables|/Script/Engine.SpringArmComponent|SetbEnableCameraLag _cameraarm (Variables|Camera|GetCameraLag?))
  (Variables|/Script/Engine.SpringArmComponent|SetCameraLagSpeed _cameraarm (Variables|Camera|GetCameraLagSpeed)))