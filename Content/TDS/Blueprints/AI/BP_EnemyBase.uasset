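; Base enemy character for the TDS game, configured from the DT_NPC data table.
; The construction script copies the NPCId row into NPCData, or sets a placeholder name and clears mesh and animation if none is found.
; BeginPlay shows the NPC name widget; animation-finish events clear the damage widget or hide and destroy the actor.
; Damage popup and death-experience logic are disconnected, and GetPhisMat is an empty stub.
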(event Custom|AnimFinish_1
  (Rendering|SetVisibility (Variables|Character|GetMesh) false false)
  (Utilities|FlowControl|Delay 1.0)
  (Actor|DestroyActor))

(event Custom|AnimFinished_Event_0
  (UserInterface|SetWidget (Variables|Default|GetDamageWidget) 0))

(event EventBeginPlay
  (bind _returnvalue (UserInterface|CreateWidget "/Game/TDS/UI/UI_Game/W_CharName.W_CharName_C"))
  (bind _output_get (Variables|Default|SetUpperWidget _returnvalue))
  (UserInterface|SetWidget (Variables|Default|GetNameWidget) _output_get)
  (Variables|/Game/TDS/UI/UI_Game/W_CharName.W_CharName_C|SetWidgetName _output_get (Utilities|Struct|BreakNPCData (Variables|Default|GetNPCData))))

(fn ConstructionScript
  (bind _mesh (Variables|Character|GetMesh))
  (bind _returnvalue (Utilities|GetDataTableRow "/Game/TDS/Blueprints/AI/DT_NPC.DT_NPC" (Variables|Default|GetNPC_Id))
    (:then
      (Variables|Default|SetNPCData (Utilities|Struct|MakeNPCData (.NPC_ID (Utilities|Struct|BreakS_NPC_Data _returnvalue)) (.WidgetName (Utilities|Struct|BreakS_NPC_Data _returnvalue)) (.SK_Mesh (Utilities|Struct|BreakS_NPC_Data _returnvalue)) (.SK_Anim (Utilities|Struct|BreakS_NPC_Data _returnvalue)) (.ComponentList (Utilities|Struct|BreakS_NPC_Data _returnvalue)) (.Mana (Utilities|Struct|BreakS_NPC_Data _returnvalue)) (.WalkSpeed (Utilities|Struct|BreakS_NPC_Data _returnvalue)) (.RunSpeed (Utilities|Struct|BreakS_NPC_Data _returnvalue)) (.bCanUseShield (Utilities|Struct|BreakS_NPC_Data _returnvalue)) (.MaxShield (Utilities|Struct|BreakS_NPC_Data _returnvalue)) (.MaxHealth (Utilities|Struct|BreakS_NPC_Data _returnvalue)) (.ShieldRecoveryValue (Utilities|Struct|BreakS_NPC_Data _returnvalue)) (.ShieldRecoveryPeriod (Utilities|Struct|BreakS_NPC_Data _returnvalue)) (.Experience (Utilities|Struct|BreakS_NPC_Data _returnvalue)) (.AnimMontage_Attack (Utilities|Struct|BreakS_NPC_Data _returnvalue)))))
    (:RowNotFound
      (Variables|Default|SetEnemyName "Unknow EnemyData NotFound")
      (Class|SkinnedMeshComponent|SetSkeletalMesh _mesh 0 true)
      (Class|SkeletalMeshComponent|SetAnimClass _mesh))))

(fn GetPhisMat
  (params (PhysMat :type Physical%20Material%20Object%20Reference))
  (return 0 0))