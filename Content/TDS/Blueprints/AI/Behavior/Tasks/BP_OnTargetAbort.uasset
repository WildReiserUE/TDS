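; Behavior tree task that resets an AI pawn, apparently when its target is aborted, by clearing focus, stopping movement and calling SetNewTarget.
; It sets walk or run by comparing the pawn's distance from the blackboard home location against the home radius, and disables orient-to-movement.
; Stationary AI rotate on tick back to their stored rotation and finish once yaw nearly matches; others finish immediately.
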(event EventReceiveExecuteAI
  (params (OwnerController :type AI%20Controller%20Object%20Reference) (ControlledPawn :type Pawn%20Object%20Reference))
  (AI|ClearFocus OwnerController)
  (AI|Navigation|StopMovement OwnerController)
  (Utilities|FlowControl|Sequence
    (:then_0
      (bind _asbp_ai_main (Utilities|Casting|CastToBP_AI_Main ControlledPawn))
      (Default|SetWalkRun _asbp_ai_main (not (CallFunction|IsToofarfromHome _asbp_ai_main)) false)
      (Default|SetNewTarget _asbp_ai_main)
      (Variables|/Script/Engine.CharacterMovementComponent|SetbOrientRotationToMovement (Variables|/Script/Engine.Character|GetCharacterMovement _asbp_ai_main) false))
    (:then_1
      (bind _asbp_ai_main_2 (Utilities|Casting|CastToBP_AI_Main ControlledPawn))
      (if (.IsStationaryAI (Default|IsStationary _asbp_ai_main_2))
        (Variables|Default|SetTargetRotation (.Rotation (Math|Transform|BreakTransform (.StationaryLocation (Default|IsStationary _asbp_ai_main_2)))))
        (Variables|Default|SetIs%20Stationary%20AI (.IsStationaryAI (Default|IsStationary _asbp_ai_main_2)))
        (else
          (AI|BehaviorTree|FinishExecute true))))))

(event EventTick
  (params (OwnerActor :type Actor%20Object%20Reference) (DeltaSeconds :type Float%20%28single-precision%29))
  (bind _targetrotation (Variables|Default|GetTargetRotation))
  (if (Variables|Default|GetIs%20Stationary%20AI)
    (Transformation|SetActorRotation (stale EventReceiveExecuteAI ControlledPawn) (Class|KismetMathLibrary|RInterptoConstant (Transformation|GetActorRotation (stale EventReceiveExecuteAI ControlledPawn)) _targetrotation DeltaSeconds 4e+02))
    (if (< (Math|Float|Absolute(Float) (.Yaw (Math|Rotator|BreakRotator (Math|Rotator|Delta(Rotator) (Transformation|GetActorRotation (stale EventReceiveExecuteAI ControlledPawn)) _targetrotation)))) 5.0)
      (AI|BehaviorTree|FinishExecute true))))

(fn IsToofarfromHome
  (params (AIRef :type Pawn%20Object%20Reference))
  (return (> (Math|Vector|VectorLength (- (Transformation|GetActorLocation AIRef) (Class|BTFunctionLibrary|GetBlackboardValueasVector (Variables|Default|GetHomeLocation)))) (Class|BTFunctionLibrary|GetBlackboardValueasFloat (Variables|Default|GetHomeRaduis)))))