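; Behavior tree task that runs a BP_AI_Main pawn to the blackboard TargetLocation while a valid Enemy is set.
; On arrival it clears UnkownDamageRunAway, picks a new target and finishes based on the Fail flag.
; Tick re-checks the target unless spooked, but its Fail assignment changes nothing and the abort logic is unwired.
; GetAwayLoc finds a debug-drawn navigable point away from a target, but this graph never calls it.
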(event EventReceiveExecuteAI
  (params (OwnerController :type AI%20Controller%20Object%20Reference) (ControlledPawn :type Pawn%20Object%20Reference))
  (bind _asbp_ai_main (Utilities|Casting|CastToBP_AI_Main ControlledPawn))
  (bind _output_get (Variables|Default|SetAIPawn _asbp_ai_main))
  (Default|SetWalkRun _output_get false false)
  (Variables|Default|SetController OwnerController)
  (bind _output_get_2 (Variables|Default|SetEnemyRef (AI|BehaviorTree|GetBlackboardValueasActor (Variables|Default|GetEnemy))))
  (Utilities|IsValid _output_get_2
    (:Is%20Valid
      (bind _output_get_3 (Variables|Default|SetNewLoc (Class|BTFunctionLibrary|GetBlackboardValueasVector (Variables|Default|GetTargetLocation))))
      (AI|AIMoveTo (Variables|Default|GetController) _output_get_3 0 5e+01 "Default" "Default" true false
        (:OnRequestFailed
          (AI|BehaviorTree|FinishExecute false))
        (:OnMoveFinished
          (Utilities|FlowControl|Sequence
            (:then_0
              (Class|BTFunctionLibrary|SetBlackboardValueasBool (Variables|Default|GetUnkownDamageRunAway) false)
              (Default|SetNewTarget (Variables|Default|GetAIPawn)))
            (:then_1
              (AI|BehaviorTree|FinishExecute (not (Variables|Default|GetFail))))))))
    (:Is%20Not%20Valid
      (AI|BehaviorTree|FinishExecute false))))

(event EventReceiveTickAI
  (params (OwnerController :type AI%20Controller%20Object%20Reference) (ControlledPawn :type Pawn%20Object%20Reference) (DeltaSeconds :type Float%20%28single-precision%29))
  (if (not (Default|IsSpookedAI (stale EventReceiveExecuteAI _output_get)))
    (if (not (Variables|Default|GetFail))
      (bind _output_get (Default|SetNewTarget (Variables|Default|GetAIPawn)))
      (if (or (!= _output_get (Variables|Default|GetEnemyRef)) (Default|IsStunned? (Variables|Default|GetAIPawn)))
        (Variables|Default|SetFail (Variables|Default|GetFail))))))

(fn GetAwayLoc
  (params (AI :type Actor%20Object%20Reference) (Target :type Actor%20Object%20Reference))
  (bind _returnvalue (Transformation|GetActorLocation AI))
  (bind _output_get (LocalVariables|SetLookaT (Math|Rotator|FindLookatRotation _returnvalue (Transformation|GetActorLocation Target))))
  (Rendering|Debug|DrawDebugSphere (+ _returnvalue (* (Math|Vector|GetForwardVector _output_get) -7.5e+02)) 3e+02 12 "(R=1.000000,G=0.000000,B=0.462350,A=1.000000)" 5.0 2.0)
  (bind (_randomlocation _returnvalue_2) (Class|NavigationSystemV1|GetRandomLocationinNavigableRadius (+ _returnvalue (* (Math|Vector|GetForwardVector _output_get) -7.5e+02)) 2e+02 0 0))
  (if _returnvalue_2
    (return _randomlocation)
    (else
      (return _returnvalue))))