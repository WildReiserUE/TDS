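; Behavior tree task that plays a random animation montage from the controlled BP_EnemyBase's NPCData montage array.
; It writes a random pick to the MontageKey blackboard entry and plays one on the mesh, with separate Random evaluations that may differ.
; It finishes successfully on montage completion, or immediately after clearing AttackAnimMontage if the array is empty.
; Failed casts and interrupted montages never call FinishExecute.
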(event EventReceiveExecuteAI
  (params (OwnerController :type AI%20Controller%20Object%20Reference) (ControlledPawn :type Pawn%20Object%20Reference))
  (bind _asbp_enemy_base (Utilities|Casting|CastToBP_EnemyBase ControlledPawn))
  (if (> (Utilities|Array|Length (Utilities|Struct|BreakNPCData (Variables|/Script/TDS.TDSAIBaseCharacter|GetNPCData _asbp_enemy_base))) 0)
    (Class|BTFunctionLibrary|SetBlackboardValueasObject (Variables|Default|GetMontageKey) (.OutItem (Utilities|Array|Random (Utilities|Struct|BreakNPCData (Variables|/Script/TDS.TDSAIBaseCharacter|GetNPCData _asbp_enemy_base)))))
    (Animation|Montage|PlayMontage (Variables|/Script/Engine.Character|GetMesh _asbp_enemy_base) (.OutItem (Utilities|Array|Random (Utilities|Struct|BreakNPCData (Variables|/Script/TDS.TDSAIBaseCharacter|GetNPCData _asbp_enemy_base))))
      (:OnCompleted
        _))
    (else
      (Variables|Default|SetAttackAnimMontage 0)))
  (AI|BehaviorTree|FinishExecute true))