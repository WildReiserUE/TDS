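; AI controller that runs a behavior tree and feeds its blackboard from perception of the player.
; On possess it starts the tree and stores the pawn's start location as HomeLocation.
; Sensing an actor tagged Player sets it as the target and cancels the forget timer.
; Any other perception update starts a ten-second timer that stops movement, clears target and flags, and sets the target location to home.
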(event OnTargetPerceptionUpdated(AiPerception)
  (params (Actor :type Actor%20Object%20Reference) (Stimulus :type AI%20Stimulus%20Structure))
  (bind _bsuccessfullysensed (Utilities|Struct|BreakAIStimulus Stimulus))
  (if (and (Actor|ActorHasTag Actor "Player") _bsuccessfullysensed)
    (AI|Components|Blackboard|SetValueasBool (Variables|Default|GetBlackboard) (Utilities|Name|MakeLiteralName "bSeePlayer") _bsuccessfullysensed)
    (Utilities|Time|ClearandInvalidateTimerbyHandle (Variables|Default|GetLookTimer))
    (bind _output_get (Variables|Default|SetActorTarget Actor))
    (Utilities|IsValid _output_get
      (:Is%20Valid
        (AI|Components|Blackboard|SetValueasObject (Variables|Default|GetBlackboard) (Utilities|Name|MakeLiteralName "TargetActor") (Variables|Default|GetActorTarget))))
    (else
      (bind _returnvalue (Utilities|Time|SetTimerbyEvent (delegate Custom|CustomEvent_0) 1e+01))
      (Variables|Default|SetLookTimer _returnvalue))))

(event Custom|CustomEvent_0
  (bind _blackboard (Variables|Default|GetBlackboard))
  (Components|Movement|StopMovementImmediately (Pawn|GetMovementComponent (Pawn|GetControlledPawn)))
  (AI|Components|Blackboard|SetValueasVector _blackboard (Utilities|Name|MakeLiteralName "TargetLocation") (AI|Components|Blackboard|GetValueasVector _blackboard (Utilities|Name|MakeLiteralName "HomeLocation")))
  (AI|Components|Blackboard|SetValueasObject (Variables|Default|GetBlackboard) (Utilities|Name|MakeLiteralName "TargetActor") 0)
  (AI|Components|Blackboard|SetValueasBool (Variables|Default|GetBlackboard) (Utilities|Name|MakeLiteralName "bSeePlayer") false)
  (AI|Components|Blackboard|SetValueasBool (Variables|Default|GetBlackboard) (Utilities|Name|MakeLiteralName "bIsInMeleeRange") false))

(event EventPossess
  (params (PossessedPawn :type Pawn%20Object%20Reference))
  (bind _returnvalue (AI|RunBehaviorTree "/Game/TDS/Blueprints/AI/AI_BehaviorTree.AI_BehaviorTree"))
  (if _returnvalue
    (AI|Components|Blackboard|SetValueasVector (Variables|Default|GetBlackboard) (Utilities|Name|MakeLiteralName "HomeLocation") (Transformation|GetActorLocation PossessedPawn))))

(fn ConstructionScript)