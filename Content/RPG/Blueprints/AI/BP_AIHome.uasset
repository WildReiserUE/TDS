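; BP_AIHome is a spawn point that fills itself with AI on the server at BeginPlay and tracks them.
; Each spawn searches randomly near the actor, using a floor trace and capsule overlap check for a clear spot.
; A gate holds party assignment until the initial spawns finish, then optionally regroups all tracked AI after each new spawn.
; Destroyed AI can return through a delayed BP_AIRespawner that references this home.
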(event Custom|OnAIDestroyed
  (params (AIClass :type BP%20AI%20Main%20Class%20Reference) (AIRef :type BP%20AI%20Main%20Object%20Reference))
  ;[1 1 1] Respawn AI
  (Utilities|Array|RemoveItem (Variables|Default|GetSpawnedAI) AIRef)
  (if (Variables|Settings|GetRespawnAI?)
    (Game|SpawnActorfromClass "/Game/RPG/Blueprints/AI/BP_AIRespawner.BP_AIRespawner_C" (Math|Transform|MakeTransform "0, 0, 0" "0, 0, 0" "1,1,1") "AdjustIfPossibleButAlwaysSpawn" 0 AIClass (Variables|Settings|GetRespawnAIDelay) self 0)))

(event Custom|Respawner_RespawnAI
  (params (Class :type BP%20AI%20Main%20Class%20Reference))
  ;[1 1 1] Respawn AI
  (bind _spawnedai (CallFunction|RespawnAI Class)))

(event Custom|OnAISpawned
  (params (AIRef :type BP%20AI%20Main%20Object%20Reference))
  (Utilities|Array|AddUnique (Variables|Default|GetSpawnedAI) AIRef)
  ;[1 1 1] Random AI spawner
  (Utilities|FlowControl|Gate false
    (:Exit
      (if (Variables|Settings|GetSetAIParty?%28ex%20Guards%29)
        (for _array_element (Variables|Default|GetSpawnedAI)
          (Default|SetAIParty _array_element (Variables|Default|GetSpawnedAI)))))))

(event EventBeginPlay
  ;[1 1 1] Random AI spawner
  (Networking|SwitchHasAuthority
    (:Authority
      (Utilities|FlowControl|Sequence
        (:then_0
          (goto _label Close))
        (:then_1
          (for _array_element (Variables|Settings|GetAIToSpawn)
            (CallFunction|RespawnAI _array_element))
          (Utilities|FlowControl|Sequence
            (:then_0
              (goto _label Open))
            (:then_1
              (Utilities|FlowControl|Gate false :!label _label
                (:Exit
                  (if (Variables|Settings|GetSetAIParty?%28ex%20Guards%29)
                    (for _array_element_2 (Variables|Default|GetSpawnedAI)
                      (Default|SetAIParty _array_element_2 (Variables|Default|GetSpawnedAI)))))))))))))

(event EventTick
  (params (DeltaSeconds :type Float%20%28single-precision%29))
  ;[1 1 1] debug
)

(fn ConstructionScript
  (Rendering|Debug|DrawDebugSphere (Transformation|GetActorLocation) (Variables|Settings|GetRaduis) 12 "(R=0.152017,G=1.000000,B=0.000000,A=1.000000)" 0.1 4.0))

(fn RespawnAI
  (params (AIClass :type BP%20AI%20Main%20Class%20Reference))
  (bind (_location _found) (CallFunction|TryGetSpawnLocation 88.0 15.0))
  (if _found
    (bind _returnvalue (Game|SpawnActorfromClass AIClass (Math|Transform|MakeTransform _location (Math|Rotator|MakeRotator 0.0 0.0 (Math|Random|RandomFloatinRange 0.0 3.6e+02)) "1,1,1") "AdjustIfPossibleButAlwaysSpawn" 0 "0.000000,0.000000,0.000000" true true self 0))
    (return _returnvalue)))

(fn TryGetSpawnLocation
  (params (CapsuleHeight :type Float%20%28single-precision%29) (Raduis :type Float%20%28single-precision%29))
  ;[1 1 1] Spawn AI, try finding a suitable spot
  (for _index (range 0 100)
    (bind _output_get (LocalVariables|SetStartingLoc (+ (Transformation|GetActorLocation) (Math|Vector|MakeVector (Math|Random|RandomFloatinRange (* (Variables|Settings|GetRaduis) -1.0) (Variables|Settings|GetRaduis)) (Math|Random|RandomFloatinRange (* (Variables|Settings|GetRaduis) -1.0) (Variables|Settings|GetRaduis)) 1e+02))))
    (bind (_outhit _returnvalue) (Collision|LineTraceByChannel _output_get (+ _output_get "0, 0,-500.000000") "TraceTypeQuery1" false 0 "None")) ; Finding the floor
    (if _returnvalue
      (bind _output_get_2 (LocalVariables|SetHitLoc (.ImpactPoint (Collision|BreakHitResult _outhit))))
      (bind (_outhit_2 _returnvalue_2) (Class|KismetSystemLibrary|CapsuleTraceSingleforObjects (+ _output_get_2 (Math|Vector|MakeVector 0.0 0.0 (+ CapsuleHeight 5.0))) (+ _output_get_2 (Math|Vector|MakeVector 0.0 0.0 (+ CapsuleHeight 5.0))) Raduis (- CapsuleHeight 5.0) (Utilities|Array|MakeArray "ObjectTypeQuery1" "ObjectTypeQuery2") false 0 "None" true "(R=1.000000,G=0.000000,B=0.000000,A=1.000000)" "(R=0.000000,G=1.000000,B=0.000000,A=1.000000)" 99.0 :!label _label))
      (if (not _returnvalue_2)
        (return (.TraceStart (Collision|BreakHitResult _outhit_2)) true))
      (else
        (LocalVariables|SetStartingLoc (+ (LocalVariables|GetStartingLoc) "0, 0,200.000000"))
        (bind (_outhit_3 _returnvalue_3) (Collision|LineTraceByChannel (LocalVariables|GetStartingLoc) (+ (LocalVariables|GetStartingLoc) "0, 0,-500.000000") "TraceTypeQuery1" false 0 "None")) ; Finding the floor
        (if _returnvalue_3
          (LocalVariables|SetHitLoc (.ImpactPoint (Collision|BreakHitResult _outhit_3)))
          (goto _label)))))
  (return "0, 0, 0" false))