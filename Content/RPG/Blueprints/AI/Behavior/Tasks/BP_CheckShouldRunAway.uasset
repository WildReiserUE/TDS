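; Behavior tree task that tells the AI whether it should run away from its blackboard enemy.
; It succeeds when the controlled BP_AI_Main reports that enemy outside its safe zone check, and fails otherwise or when references are invalid.
; A GetAwayLoc helper, not called in this graph, picks a random navigable point behind the AI, facing away from the target, and draws a debug sphere.
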(event EventReceiveExecuteAI
  (params (OwnerController :type AI%20Controller%20Object%20Reference) (ControlledPawn :type Pawn%20Object%20Reference))
  (bind _output_get (Variables|Default|SetEnemyRef (AI|BehaviorTree|GetBlackboardValueasActor (Variables|Default|GetEnemy))))
  (Utilities|IsValid _output_get
    (:Is%20Valid
      (bind _asbp_ai_main (Utilities|Casting|CastToBP_AI_Main ControlledPawn)
        (:then
          (AI|BehaviorTree|FinishExecute (not (Default|IsTargetWithinSafeZone _asbp_ai_main (Variables|Default|GetEnemyRef)))))
        (:CastFailed
          (AI|BehaviorTree|FinishExecute false :!label _label))))
    (:Is%20Not%20Valid
      (goto _label))))

(fn GetAwayLoc
  (params (AI :type Actor%20Object%20Reference) (Target :type Actor%20Object%20Reference))
  (bind _returnvalue (Transformation|GetActorLocation AI))
  (bind _output_get (LocalVariables|SetLookaT (Math|Rotator|FindLookatRotation _returnvalue (Transformation|GetActorLocation Target))))
  (Rendering|Debug|DrawDebugSphere (+ _returnvalue (* (Math|Vector|GetForwardVector _output_get) -7.5e+02)) 3e+02 12 "(R=1.000000,G=0.000000,B=0.462350,A=1.000000)" 5.0 2.0)
  (bind (_randomlocation _returnvalue_2) (Class|NavigationSystemV1|GetRandomLocationinNavigableRadius (+ _returnvalue (* (Math|Vector|GetForwardVector _output_get) -7.5e+02)) 2e+02 0 0))
  (if _returnvalue_2
    (return _randomlocation)
    (else
      (return _returnvalue))))