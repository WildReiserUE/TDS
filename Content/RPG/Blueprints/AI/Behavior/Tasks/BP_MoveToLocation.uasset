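; Behavior tree task that moves an AI character to the blackboard's TargetLocation.
; On execute it fails if the BP_AI_Main pawn is stunned, otherwise runs AI MoveTo and reports the move's success or failure.
; While ticking, for one specific hostility and behavior combination, it searches for a new target and finishes successfully early if one is found, so the AI can react to nearby threats.
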(event EventReceiveExecuteAI
  (params (OwnerController :type AI%20Controller%20Object%20Reference) (ControlledPawn :type Pawn%20Object%20Reference))
  (bind _asbp_ai_main (Utilities|Casting|CastToBP_AI_Main ControlledPawn))
  (if (Default|IsStunned? _asbp_ai_main)
    (AI|BehaviorTree|FinishExecute false)
    (else
      (AI|AIMoveTo OwnerController (Class|BTFunctionLibrary|GetBlackboardValueasVector (Variables|Default|GetTargetLocation)) 0 5e+01 "Default" "Default" true false
        (:OnRequestFailed
          (AI|BehaviorTree|FinishExecute false))
        (:OnMoveFinished
          (AI|BehaviorTree|FinishExecute true))))))

(event EventReceiveTickAI
  (params (OwnerController :type AI%20Controller%20Object%20Reference) (ControlledPawn :type Pawn%20Object%20Reference) (DeltaSeconds :type Float%20%28single-precision%29))
  ;[1 1 1] Since AI can still spot a threat it will only react if the threat is close enough therefore this checks for a threat every 0.25 sec
  (if (and (Utilities|Enum|Equal(Enum) (Utilities|Enum|ByteToEnumE_AIHostilityType (Class|BTFunctionLibrary|GetBlackboardValueasEnum (Variables|Default|GetAIHostility))) "NewEnumerator5") (Utilities|Enum|Equal(Enum) (Utilities|Enum|ByteToEnumE_AIBehaviorType (Class|BTFunctionLibrary|GetBlackboardValueasEnum (Variables|Default|GetBehavior))) "NewEnumerator6"))
    (bind _output_get (Default|SetNewTarget (stale EventReceiveExecuteAI _asbp_ai_main)))
    (Utilities|IsValid _output_get
      (:Is%20Valid
        (AI|BehaviorTree|FinishExecute true)))))