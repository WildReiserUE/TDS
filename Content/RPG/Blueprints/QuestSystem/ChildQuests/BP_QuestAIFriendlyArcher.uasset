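; BP_QuestAIFriendlyArcher is a quest AI archer that turns into an ally of the player when a quest completes.
; Construction runs the parent script, then slaves the armor and arms meshes to the main mesh's pose.
; On quest completion it activates its AI, marks the player as friendly, changes its hostility, and makes its capsule ignore the Visibility trace channel.
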(fn ConstructionScript
  (|CallParentFunction)
  (Class|SkinnedMeshComponent|SetMasterPoseComponent (Variables|Default|GetArmor_0) (Variables|Character|GetMesh) false))

(fn OnQuestCompleted
  (params (Player :type Actor%20Object%20Reference) (QuestUID :type Name :default "None"))
  (CallFunction|ActivateAI)
  (CallFunction|SetFriendlyActor Player)
  (CallFunction|SetHostility "NewEnumerator0")
  (Collision|SetCollisionResponsetoChannel (Variables|Default|GetCapsuleComponent) "ECC_Visibility" "ECR_Ignore"))