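; A skill zone actor that heavily slows the movement of actors while they are inside its box volume.
; On begin overlap, the server adds an infinite, apply-once "SlowMov" effect to the actor's BP_SkillEffectsComponent.
; On end overlap, the server removes that effect by ID, so actors without the component are unaffected and the slow lasts only while overlapping.
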(event OnComponentBeginOverlap(Box)
  (params (OverlappedComponent :type Primitive%20Component%20Object%20Reference) (OtherActor :type Actor%20Object%20Reference) (OtherComp :type Primitive%20Component%20Object%20Reference) (OtherBodyIndex :type Integer) (bFromSweep :type Boolean) (SweepResult :type Hit%20Result%20Structure%20%28by%20ref%29))
  (Networking|SwitchHasAuthority
    (:Authority
      (bind _output_get (Variables|Default|SetComp (Actor|GetComponentbyClass OtherActor "/Game/RPG/Blueprints/Components/BP_SkillEffectsComponent.BP_SkillEffectsComponent_C")))
      (Utilities|IsValid _output_get
        (:Is%20Valid
          (Default|AddNewEffect _output_get self (Utilities|Struct|MakeS_SkillEffects "SlowMov" "NewEnumerator1" 1e+02 true 0.0 -1.0 0.0 "/Game/RPG/Blueprints/Skills/DamageTypes/BP_PhysicalDamage.BP_PhysicalDamage_C" 0.0 0.0 0.0 0.0 -75.0)))))))

(event OnComponentEndOverlap(Box)
  (params (OverlappedComponent :type Primitive%20Component%20Object%20Reference) (OtherActor :type Actor%20Object%20Reference) (OtherComp :type Primitive%20Component%20Object%20Reference) (OtherBodyIndex :type Integer))
  (Networking|SwitchHasAuthority
    (:Authority
      (bind _output_get (Variables|Default|SetComp (Actor|GetComponentbyClass OtherActor "/Game/RPG/Blueprints/Components/BP_SkillEffectsComponent.BP_SkillEffectsComponent_C")))
      (Utilities|IsValid _output_get
        (:Is%20Valid
          (Default|RemoveEffectbyID _output_get "SlowMov"))))))

(fn ConstructionScript)