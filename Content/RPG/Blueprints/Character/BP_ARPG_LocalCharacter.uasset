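; Local top-down RPG character that acts as a stand-in for an owning character, copying its mesh and capsule and ignoring it when moving.
; AI controller moves drive it to locations or actors; tick handles turning toward targets and eases spring arm length.
; It snaps or delay-corrects to the owner's transform, handles stun, launch and teleport, and ragdolls on death, restoring the mesh on revive.
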(event Custom|MoveToLocation
  (params (Dest :type Vector%20%28by%20ref%29) (AcceptanceRadius :type Float%20%28single-precision%29))
  ;[1 1 1] Move to location
  (bind _returnvalue (AI|Navigation|MovetoLocation (AI|GetAIController self) Dest AcceptanceRadius false true false true 0))
  (if (Utilities|Enum|Equal(Enum) _returnvalue "AlreadyAtGoal")
    (Variables|Default|SetTargetRot (Math|Rotator|MakeRotator 0.0 0.0 (.yaw (Math|Rotator|FindLookatRotation (Transformation|GetActorLocation) Dest))))
    (Variables|Default|SetDoTarget true)
    (else
      (Variables|Default|SetDoTarget false))))

(event Custom|MoveToActor
  (params (Target :type Actor%20Object%20Reference) (CustomRange :type Float%20%28single-precision%29))
  ;[1 1 1] Move to actor
  (bind _distance (Class|BPIInteract|GetAcceptableDistance(Message) Target))
  (bind _returnvalue (AI|Navigation|MovetoActor (AI|GetAIController self) Target (Math|Float|SelectFloat (Math|Float|SelectFloat _distance 5e+01 (> _distance 0.0)) CustomRange (< CustomRange 0.0)) false true true 0))
  (if (Utilities|Enum|Equal(Enum) _returnvalue "AlreadyAtGoal")
    (Variables|Default|SetTargetRot (Math|Rotator|MakeRotator 0.0 0.0 (.yaw (Math|Rotator|FindLookatRotation (Transformation|GetActorLocation) (Transformation|GetActorLocation Target)))))
    (Variables|Default|SetDoTarget true)
    (else
      (Variables|Default|SetDoTarget false))))

(event Custom|SetTargetLen
  (params (TargetLen :type Float%20%28single-precision%29))
  ;[1 1 1] Rotation and spring arm
  (Variables|Default|SetTargetLen TargetLen))

(event Custom|DelayedCorrectPosition
  ;[1 1 1] Correct position
  (Utilities|FlowControl|RetriggerableDelay 5.0)
  (CallFunction|CorrectPosition))

(event EventTick
  (params (DeltaSeconds :type Float%20%28single-precision%29))
  ;[1 1 1] Rotation and spring arm
  (CallFunction|HandleTargeting DeltaSeconds)
  (Variables|/Script/Engine.SpringArmComponent|SetTargetArmLength (Variables|Default|GetTopDownSpring) (Math|Interpolation|FInterpTo (Variables|/Script/Engine.SpringArmComponent|GetTargetArmLength (Variables|Default|GetTopDownSpring)) (Variables|Default|GetTargetLen) DeltaSeconds 5.0)))

(fn ConstructionScript
  (|CallParentFunction)
  (Variables|Default|SetDefaultMeshT (Transformation|GetRelativeTransform (Variables|Character|GetMesh)))
  (Variables|Default|SetTargetLen (Variables|/Script/Engine.SpringArmComponent|GetTargetArmLength (Variables|Default|GetTopDownSpring))))

(fn GetMesh
  (return (Variables|Character|GetMesh)))

(fn HandleTargeting
  (params (Delta :type Float%20%28single-precision%29))
  (if (Variables|Default|GetDoTarget)
    (Transformation|SetActorRotation (Class|KismetMathLibrary|RInterptoConstant (Transformation|GetActorRotation) (Variables|Default|GetTargetRot) Delta 7.5e+02) true)
    (if (< (Math|Float|Absolute(Float) (.yaw (Math|Rotator|Delta(Rotator) (Transformation|GetActorRotation) (Variables|Default|GetTargetRot)))) 2.0)
      (Variables|Default|SetDoTarget false))))

(fn OnPlayerStunned
  (params (IsPlayerStunned :type Boolean))
  (if IsPlayerStunned
    (Components|Movement|StopMovementImmediately (Variables|Character|GetCharacterMovement))
    (Variables|Default|SetDoTarget false)))

(fn StopMovement
  (Components|Movement|StopMovementImmediately (Variables|Character|GetCharacterMovement))
  (Variables|Default|SetDoTarget false))

(fn OnPlayerAlive
  (params (IsAlive :type Boolean))
  (bind _characterowner (Variables|Default|GetCharacterOwner))
  (bind _mesh (Variables|Character|GetMesh))
  (if IsAlive
    (Class|SkeletalMeshComponent|SetAllBodiesSimulatePhysics (Variables|Character|GetMesh) false)
    (Collision|SetCollisionResponsetoChannel (Variables|Collision|GetCapsuleComponent) "ECC_Pawn" "ECR_Block")
    (Transformation|AttachComponentToComponent _mesh (Variables|Collision|GetCapsuleComponent) "None" "SnapToTarget" "SnapToTarget" "SnapToTarget" true)
    (Transformation|SetRelativeTransform _mesh (Variables|Default|GetDefaultMeshT) false true)
    (Transformation|SetActorLocationAndRotation (Transformation|GetActorLocation _characterowner) (Transformation|GetActorRotation _characterowner) false true)
    (else
      (Components|Movement|StopMovementImmediately (Variables|Character|GetCharacterMovement))
      (Animation|StopAnimMontage 0)
      (Class|SkeletalMeshComponent|SetAllBodiesBelowSimulatePhysics (Variables|Character|GetMesh) (Utilities|Name|MakeLiteralName "pelvis") true true)
      (Collision|SetCollisionResponsetoChannel (Variables|Collision|GetCapsuleComponent) "ECC_Pawn" "ECR_Ignore"))))

(fn GetHealthbar
  (return (.AsBP%20AIHealthbar (Utilities|Casting|CastToBP_AIHealthbar (UserInterface|GetUserWidgetObject (Variables|Default|GetWidget))))))

(fn SetTarget
  (params (TargetRot :type Rotator))
  (Variables|Default|SetTargetRot (Math|Rotator|MakeRotator 0.0 0.0 (.yaw TargetRot)))
  (Variables|Default|SetDoTarget true))

(fn SetMovementSpeed
  (params (WalkSpeed :type Float%20%28single-precision%29) (Debuff :type Float%20%28single-precision%29))
  (Variables|/Script/Engine.CharacterMovementComponent|SetMaxWalkSpeed (Variables|Character|GetCharacterMovement) (+ (* WalkSpeed Debuff) WalkSpeed)))

(fn SetCharacterOwner
  (params (CharacterOwner :type Pawn%20Object%20Reference))
  (bind _output_get (Variables|Default|SetCharacterOwner CharacterOwner))
  (Collision|IgnoreActorwhenMoving (Variables|Collision|GetCapsuleComponent) _output_get true))

(fn SetMesh
  (params (MeshComponent :type Skeletal%20Mesh%20Component%20Object%20Reference) (Capsule :type Capsule%20Component%20Object%20Reference))
  (bind _capsulecomponent (Variables|Collision|GetCapsuleComponent))
  (Class|SkinnedMeshComponent|SetSkeletalMesh (Variables|Character|GetMesh) (Variables|/Script/Engine.SkinnedMeshComponent|GetSkeletalMesh MeshComponent) false)
  (for (_array_element _array_index) (Rendering|Material|GetMaterials MeshComponent)
    (Rendering|Material|SetMaterial (Variables|Character|GetMesh) _array_index _array_element))
  (Class|SkeletalMeshComponent|SetAnimClass (Variables|Character|GetMesh) (Variables|/Script/Engine.SkeletalMeshComponent|GetAnimClass MeshComponent))
  (Components|Capsule|SetCapsuleRadius _capsulecomponent (Variables|/Script/Engine.CapsuleComponent|GetCapsuleRadius Capsule) true)
  (Components|Capsule|SetCapsuleHalfHeight _capsulecomponent (Variables|/Script/Engine.CapsuleComponent|GetCapsuleHalfHeight Capsule) true)
  (Transformation|SetRelativeLocationAndRotation (Variables|Character|GetMesh) (Variables|/Script/Engine.SceneComponent|GetRelativeLocation MeshComponent) (Variables|/Script/Engine.SceneComponent|GetRelativeRotation MeshComponent) false true))

(fn CorrectPosition
  (bind _characterowner (Variables|Default|GetCharacterOwner))
  (Transformation|SetActorLocationAndRotation (Transformation|GetActorLocation _characterowner) (Transformation|GetActorRotation _characterowner) false true))

(fn TeleportPlayer
  (params (NewLocation :type Vector) (NewRotation :type Rotator) (bTeleport :type Boolean))
  (Components|Movement|StopMovementImmediately (Variables|Character|GetCharacterMovement))
  (Transformation|SetActorLocationAndRotation NewLocation NewRotation false bTeleport))

(fn LaunchLocalPlayer
  (params (LaunchVelocity :type Vector) (bXYOverride :type Boolean) (bZOverride :type Boolean))
  (Components|Movement|StopMovementImmediately (Variables|Character|GetCharacterMovement))
  (Character|LaunchCharacter LaunchVelocity bXYOverride bZOverride))

(fn GetEquippedInfo
  (bind _characterowner (Variables|Default|GetCharacterOwner))
  (Utilities|IsValid _characterowner
    (:Is%20Valid
      (bind (_primary _secondary) (Class|BPIAnimationInfo|GetEquippedInfo(Message) _characterowner))
      (return _primary _secondary))
    (:Is%20Not%20Valid
      (return "" ""))))