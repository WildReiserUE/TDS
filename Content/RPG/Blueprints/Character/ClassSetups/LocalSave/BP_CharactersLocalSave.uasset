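; Save game object that stores the list of locally saved RPG characters, with class, race, gender, name, level, main equipment and map.
; It adds entries to the SavedCharacters array and looks them up, checks or deletes them by character name.
; Level, equipment and map are updated by unique ID instead of name.
; SaveToSlot writes the object itself to the fixed RPG_LocalChars slot.
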(fn DoesNameExist
  (params (Name :type String))
  (for _array_element (Variables|Default|GetSavedCharacters)
    (if (Utilities|Enum|Equal(Enum) (.CharacterName (Utilities|Struct|BreakS_SavedLocalCharacter _array_element)) Name)
      (return true)))
  (return false))

(fn AddNewCharacter
  (params (UniqueID :type Integer) (ClassType :type E_ClassTypes%20Enum :default "NewEnumerator0") (RaceType :type E_RaceType%20Enum :default "NewEnumerator6") (GenderType :type E_GenderType%20Enum :default "NewEnumerator2") (ClassName :type Name) (CharacterName :type String) (Level :type Integer) (MainEquipment :type Array%20of%20S%20Starting%20Items%20Structures))
  (Utilities|Array|Add (Variables|Default|GetSavedCharacters) (Utilities|Struct|MakeS_SavedLocalCharacter UniqueID ClassType RaceType GenderType ClassName CharacterName Level "" MainEquipment)))

(fn GetCharacterbyName
  (params (Name :type String))
  (for _array_element (Variables|Default|GetSavedCharacters)
    (if (Utilities|Enum|Equal(Enum) (.CharacterName (Utilities|Struct|BreakS_SavedLocalCharacter _array_element)) Name)
      (return true _array_element)))
  (return false ""))

(fn DeleteCharacterbyName
  (params (Name :type String))
  (for (_array_element _array_index) (Variables|Default|GetSavedCharacters)
    (if (Utilities|Enum|Equal(Enum) (.CharacterName (Utilities|Struct|BreakS_SavedLocalCharacter _array_element)) Name)
      (Utilities|Array|RemoveIndex (Variables|Default|GetSavedCharacters) _array_index)
      (return true)))
  (return false))

(fn SavetoSlot
  (SaveGame|SaveGametoSlot self "RPG_LocalChars"))

(fn UpdateInfobyUID
  (params (UID :type Integer) (Level :type Integer) (MainEquipment :type Array%20of%20S%20Starting%20Items%20Structures) (MapName :type String))
  (for (_array_element _array_index) (Variables|Default|GetSavedCharacters)
    (if (== (Utilities|Struct|BreakS_SavedLocalCharacter _array_element) UID)
      (Utilities|Struct|SetmembersinS_SavedLocalCharacter (Utilities|Array|Get(acopy) (Variables|Default|GetSavedCharacters) _array_index) Level MapName MainEquipment))))