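; BP_DamageTaken is an actor that shows a floating combat number for damage or healing.
; On BeginPlay it passes its damage amount, color, damage type and healed flag to the user widget of its Widget component.
; Tick moves that component upward at a constant speed and destroys the actor once its relative height passes a fixed threshold.
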(event EventBeginPlay
  (bind _asbp_damage_taken (Utilities|Casting|CastToBP_DamageTaken (UserInterface|GetUserWidgetObject (Variables|Default|GetWidget))))
  (Default|SetDamage _asbp_damage_taken (Variables|Default|GetDamage) (Variables|Default|GetColor) (Variables|Default|GetDmgType) (Variables|Default|GetHealed?)))

(event EventTick
  (params (DeltaSeconds :type Float%20%28single-precision%29))
  (Transformation|AddWorldOffset (Variables|Default|GetWidget) (Math|Vector|MakeVector 0.0 0.0 (* DeltaSeconds 2e+02)) false true)
  (if (> (.z (Variables|/Script/Engine.SceneComponent|GetRelativeLocation (Variables|Default|GetWidget))) 1e+02)
    (Actor|DestroyActor)))

(fn ConstructionScript)